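; BP_ItemBase is a base item actor that can sit in the world or inside a container component.
; It derives stackability, fullness and stack weight from its BasicInfo and quantity, which is fixed at one here.
; Entering a container attaches the hidden actor to the container's owner and records that component; returning to the world detaches and reveals it.
; Initialize, Interact and SetQuantity are stubs that return true.
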(fn `GetBasicInfo`
  (returns (ReturnValue :type "ItemBasicInfo Structure"))
  (return (`self.BasicInfo`)))

(fn `GetIsStackFull`
  (returns (ReturnValue :type Boolean))
  (bind (_returnvalue_name _returnvalue_description _returnvalue_weight _returnvalue_maxstacksize) (break `ItemBasicInfo` (`ItemInterface.GetBasicInfo`)))
  (return (>= (`ItemInterface.GetQuantity`) _returnvalue_maxstacksize)))

(fn `GetOwningContainerComponent`
  (returns (ReturnValue :type "ContainerComponent Object Reference"))
  (return (`self.OwningContainerComponent`)))

(fn `GetQuantity`
  (returns (ReturnValue :type Integer))
  (return 1))

(fn `GetStackable`
  (returns (ReturnValue :type Boolean))
  (bind (_returnvalue_name _returnvalue_description _returnvalue_weight _returnvalue_maxstacksize) (break `ItemBasicInfo` (`ItemInterface.GetBasicInfo`)))
  (return (> _returnvalue_maxstacksize 1)))

(fn `GetStackWeight`
  (returns (ReturnValue :type "Float (single-precision)"))
  (bind (_returnvalue_name _returnvalue_description _returnvalue_weight) (break `ItemBasicInfo` (`ItemInterface.GetBasicInfo`)))
  (return (* _returnvalue_weight (`ItemInterface.GetQuantity`))))

(fn `Initialize`
  (params (bIsInContainer :type Boolean))
  (returns (ReturnValue :type Boolean))
  (return true))

(fn `Interact`
  (params (Instigator :type "Pawn Object Reference"))
  (returns (ReturnValue :type Boolean))
  (return true))

(fn `OnAddedToContainer`
  (params (TargetContainer :type "ContainerComponent Object Reference"))
  (returns (ReturnValue :type Boolean))
  (bind _returnvalue (`ActorComponent.GetOwner` TargetContainer))
  (`|ExecutionSequence`
    (:`then_0`
      (`/Engine/EditorBlueprintResources/StandardMacros.IsValid` TargetContainer
        (:`Is Valid`
          (`/Engine/EditorBlueprintResources/StandardMacros.IsValid` _returnvalue
            (:`Is Valid`
              (`self.K2_AttachToActor` _returnvalue "None" "SnapToTarget" "SnapToTarget" "KeepRelative")
              (`SceneComponent.SetVisibility` (`self.DefaultSceneRoot`) false true)
              (set `self.OwningContainerComponent` TargetContainer)
              (return true))))))
    (:`then_1`
      (return false))))

(fn `OnAddedToWorld`
  (returns (ReturnValue :type Boolean))
  (`self.K2_DetachFromActor` "KeepWorld" "KeepWorld" "KeepWorld")
  (`SceneComponent.SetVisibility` (`self.DefaultSceneRoot`) true true)
  (return true))

(fn `SetQuantity`
  (params (TargetQuantity :type Integer))
  (returns (ReturnValue :type Boolean))
  (return true))

(fn `UserConstructionScript`)